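; BP_Interact is an actor with a widget component that appears while its IsLooking flag is true.
; While visible, it gets the BP_FirstPersonCharacter each Tick and smoothly turns only its yaw toward that player using FindLookAtRotation and RInterpTo.
; When the flag is false, Tick hides the widget; nothing in this graph sets the flag.
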(event Custom|Lookatplayer
  (Transformation|SetActorRotation (Math|Rotator|MakeRotator 0.0 0.0 (.yaw (Math|Interpolation|RInterpTo (Transformation|GetActorRotation) (Math|Rotator|FindLookatRotation (Transformation|GetActorLocation self) (Transformation|GetActorLocation (stale EventTick _returnvalue))) (Utilities|Time|GetWorldDeltaSeconds) 2e+01)))))

(event EventTick
  (params (DeltaSeconds :type Float%20%28single-precision%29))
  (if (Variables|Default|GetisLooking)
    (Rendering|SetVisibility (Variables|Default|GetWidget) true false)
    (bind _returnvalue (Actor|GetActorOfClass "/Game/FirstPerson/Blueprints/BP_FirstPersonCharacter.BP_FirstPersonCharacter_C"))
    (CallFunction|Lookatplayer)
    (else
      (Rendering|SetVisibility (Variables|Default|GetWidget) false false))))

(fn ConstructionScript)