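; BP_Door is an interactable door that toggles between open and closed through its Interact function.
; Interact flips IsOpen and calls the open or close event, which plays or reverses one timeline.
; The timeline drives the actor's absolute roll and world Z height, keeping its other rotation and location components.
; Opening plays a 2D sound, closing only prints a debug string, and Interact always returns false.
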(event Custom|DoorInteractOpen
  (bind _returnvalue (Transformation|GetActorLocation))
  (bind _returnvalue_2 (Transformation|GetActorRotation))
  (bind (_direction _position _rotation) (Timeline|Timeline_0 Play)
    (:Update
      (Transformation|SetActorRotation (Math|Rotator|MakeRotator _rotation (.pitch _returnvalue_2) (.yaw _returnvalue_2)))
      (Transformation|SetActorLocation (Math|Vector|MakeVector (.x _returnvalue) (.y _returnvalue) _position) false false))))

(event Custom|DoorInteractClose
  (bind _returnvalue (Transformation|GetActorLocation))
  (bind _returnvalue_2 (Transformation|GetActorRotation))
  (bind (_direction _position _rotation) (Timeline|Timeline_0 Reverse)
    (:Update
      (Transformation|SetActorRotation (Math|Rotator|MakeRotator _rotation (.pitch _returnvalue_2) (.yaw _returnvalue_2)))
      (Transformation|SetActorLocation (Math|Vector|MakeVector (.x _returnvalue) (.y _returnvalue) _position) false false))))

(fn ConstructionScript)

(fn Interact
  (params (Player :type Character%20Object%20Reference))
  (if (Variables|Default|GetisOpen)
    (CallFunction|DoorInteractClose)
    (Variables|Default|SetisOpen false)
    (Development|PrintString "Door closing")
    (else
      (CallFunction|DoorInteractOpen)
      (Variables|Default|SetisOpen true)
      (Audio|PlaySound2D "/Game/_Anthony/Audio/431117__inspectorj__door-front-opening-a.431117__inspectorj__door-front-opening-a" 1.0 1.0 0.0 0 0)))
  (return false))